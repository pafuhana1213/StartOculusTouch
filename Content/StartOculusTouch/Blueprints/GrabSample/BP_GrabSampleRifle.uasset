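; Grabbable VR sample rifle that fires automatically while used, spawning bullets at the muzzle with a haptic pulse per shot.
; BPCGrabTarget delegates drive grab, release, use and targeting highlight; button and thumbstick handlers are empty.
; Grabbing snaps it to the controller using the inverted grab-target offset and makes any other holding hand release; releasing detaches it into physics.
; A Gate with a Delay loop repeats shots until use stops.
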(event Custom|StopUsed
  (params (MotionController :type BP%20Motion%20Controller%20Object%20Reference))
  ;[1 1 1] Stop Used
  (Default|SetHapticsbyValue MotionController 3.2e+02 0.0)
  ;[1 1 1] Start Used
  (Utilities|FlowControl|Gate true) ; enters at Close
)

(event Custom|Grabed
  (params (MotionController :type BP%20Motion%20Controller%20Object%20Reference))
  (bind _bpc_grabtarget (Variables|Default|GetBPC_GrabTarget))
  (bind _returnvalue (Transformation|GetRelativeTransform _bpc_grabtarget))
  (bind _returnvalue_2 (Math|Transform|InvertTransform _returnvalue))
  ;[1 1 1] Grabed
  (Utilities|FlowControl|Sequence
    (:then_0
      (bind _isexchange (CallFunction|CheckExchange MotionController))
      (if _isexchange
        (CallFunction|StopUsed MotionController)))
    (:then_1
      (bind _output_get (Variables|Default|SetGrabMotionController MotionController))
      (Transformation|AttachActorToActor _output_get "None" "SnapToTarget" "SnapToTarget" "KeepRelative" true)
      (Class|Actor|AddActorLocalTransform (Math|Transform|MakeTransform (.location _returnvalue_2) (.rotation _returnvalue_2) "1.000000,1.000000,1.000000") false false))))

(event Custom|Released
  (params (MotionController :type BP%20Motion%20Controller%20Object%20Reference))
  ;[1 1 1] Released
  (Utilities|FlowControl|Sequence
    (:then_0
      (Transformation|DetachFromActor "KeepRelative" "KeepRelative" "KeepRelative")
      (Variables|Default|SetGrabMotionController 0)
      (Physics|SetSimulatePhysics (Variables|Default|GetSkeletalMesh) true))
    (:then_1
      (CallFunction|StopUsed MotionController))))

(event Custom|Shot
  (bind _grabmotioncontroller (Variables|Default|GetGrabMotionController))
  ;[1 1 1] Shot
  (Game|SpawnActorfromClass "/Game/StartOculusTouch/Blueprints/GrabSample/BP_Bullet.BP_Bullet_C" (Transformation|GetWorldTransform (Variables|Default|GetMuzzle)) "Undefined" 0 0)
  (Default|SetHapticsbyValue _grabmotioncontroller 3.2e+02 1.0)
  (Utilities|FlowControl|Delay 0.05)
  (Utilities|IsValid _grabmotioncontroller
    (:Is%20Valid
      (Default|SetHapticsbyValue _grabmotioncontroller 3.2e+02 0.0))))

(event Custom|StartUsed
  (params (MotionController :type BP%20Motion%20Controller%20Object%20Reference))
  ;[1 1 1] Start Used
  (Utilities|FlowControl|Sequence
    (:then_0
      (goto _label Open))
    (:then_1
      (Utilities|FlowControl|Gate true :!label _label
        (:Exit
          (CallFunction|Shot)
          (Utilities|FlowControl|Delay 0.1)
          (goto _label))))))

(event Custom|PressButton1
  (params (MotionController :type BP%20Motion%20Controller%20Object%20Reference))
  ;[1 1 1] Button 1
)

(event Custom|ReleaseButton1
  (params (MotionController :type BP%20Motion%20Controller%20Object%20Reference))
  ;[1 1 1] Button 1
)

(event Custom|Targeted
  (params (MotionController :type BP%20Motion%20Controller%20Object%20Reference))
  ;[1 1 1] Targeted
  (Rendering|Material|SetScalarParameterValue (Variables|Default|GetMaterial) "IsTargeted" 1.0 :!class /Script/Engine.MaterialInstanceDynamic))

(event Custom|PressButton2
  (params (MotionController :type BP%20Motion%20Controller%20Object%20Reference))
  ;[1 1 1] Button 2
)

(event Custom|NotTargeted
  (params (MotionController :type BP%20Motion%20Controller%20Object%20Reference))
  ;[1 1 1] Not Targeted
  (Rendering|Material|SetScalarParameterValue (Variables|Default|GetMaterial) "IsTargeted" 0.0 :!class /Script/Engine.MaterialInstanceDynamic))

(event Custom|ReleaseButton2
  (params (MotionController :type BP%20Motion%20Controller%20Object%20Reference))
  ;[1 1 1] Button 2
)

(event Custom|PressThumbStick
  (params (MotionController :type BP%20Motion%20Controller%20Object%20Reference))
  ;[1 1 1] ThumbStick
)

(event Custom|ReleaseThumbStick
  (params (MotionController :type BP%20Motion%20Controller%20Object%20Reference))
  ;[1 1 1] ThumbStick
)

(event Custom|Bind%20Grabed
  ;[1 1 1] Grabed
  (EventDispatchers|AssignEDGrabed (Variables|Default|GetBPC_GrabTarget) (delegate Custom|Grabed)))

(event EventBeginPlay
  ;[1 1 1] BeginPlay
  (CallFunction|BindEvents))

(fn ConstructionScript
  (bind _returnvalue (Rendering|Material|CreateDynamicMaterialInstance (Variables|Default|GetSkeletalMesh) 0 "/Game/StartOculusTouch/Material/M_GrabTarget.M_GrabTarget" :!class /Script/Engine.PrimitiveComponent))
  (Variables|Default|SetMaterial _returnvalue))

(fn CheckExchange
  (params (MotionController :type BP%20Motion%20Controller%20Object%20Reference))
  (bind _grabmotioncontroller (Variables|Default|GetGrabMotionController))
  (if (and (!= MotionController _grabmotioncontroller) (Utilities|IsValid _grabmotioncontroller))
    (Default|ReleasebyOtherHand (Variables|Default|GetGrabMotionController))
    (return true)
    (else
      (return false))))

(fn BindEvents
  (bind _bpc_grabtarget (Variables|Default|GetBPC_GrabTarget))
  (bind _bpc_grabtarget_2 (Variables|Default|GetBPC_GrabTarget))
  (bind _bpc_grabtarget_3 (Variables|Default|GetBPC_GrabTarget))
  (bind _bpc_grabtarget_4 (Variables|Default|GetBPC_GrabTarget))
  (bind _bpc_grabtarget_5 (Variables|Default|GetBPC_GrabTarget))
  (bind _bpc_grabtarget_6 (Variables|Default|GetBPC_GrabTarget))
  (Utilities|FlowControl|Sequence
    (:then_0
      ;[1 1 1] Grab / Release
      (EventDispatchers|BindEventtoEDGrabed _bpc_grabtarget_3 (EventDispatchers|CreateEvent :!event Custom|Grabed))
      (EventDispatchers|BindEventtoEDReleased _bpc_grabtarget_3 (EventDispatchers|CreateEvent :!event Custom|Released))
      ;[1 1 1] Targeted
      (EventDispatchers|BindEventtoEDTargeted _bpc_grabtarget (EventDispatchers|CreateEvent :!event Custom|Targeted))
      (EventDispatchers|BindEventtoEDNotTargeted _bpc_grabtarget (EventDispatchers|CreateEvent :!event Custom|NotTargeted))
      ;[1 1 1] Used
      (EventDispatchers|BindEventtoEDStartUsed _bpc_grabtarget_2 (EventDispatchers|CreateEvent :!event Custom|StartUsed))
      (EventDispatchers|BindEventtoEDStopUsed _bpc_grabtarget_2 (EventDispatchers|CreateEvent :!event Custom|StopUsed)))
    (:then_1
      ;[1 1 1] Thumb Stick
      (EventDispatchers|BindEventtoEDPressThumbStick _bpc_grabtarget_4 (EventDispatchers|CreateEvent :!event Custom|PressThumbStick))
      (EventDispatchers|BindEventtoEDReleaseThumbStick _bpc_grabtarget_4 (EventDispatchers|CreateEvent :!event Custom|ReleaseThumbStick))
      ;[1 1 1] Button 1
      (EventDispatchers|BindEventtoEDPressButton1 _bpc_grabtarget_5 (EventDispatchers|CreateEvent :!event Custom|PressButton1))
      (EventDispatchers|BindEventtoEdReleaseButton1 _bpc_grabtarget_5 (EventDispatchers|CreateEvent :!event Custom|ReleaseButton1))
      ;[1 1 1] Button2
      (EventDispatchers|BindEventtoEDPressButton2 _bpc_grabtarget_6 (EventDispatchers|CreateEvent :!event Custom|PressButton2))
      (EventDispatchers|BindEventtoEDReleaseButton2 _bpc_grabtarget_6 (EventDispatchers|CreateEvent :!event Custom|ReleaseButton2)))))
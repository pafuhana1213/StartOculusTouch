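; BP_MotionController is an Oculus Touch VR hand that targets, grabs and releases actors with a BPC_GrabTarget component.
; Each tick it aims the grab box along the camera-to-hand line and targets the nearest overlapping component.
; Grabbing hides the hand mesh and forwards use, button and stick-press events to the held component.
; It also stores touch input state, plays per-hand haptics and mirrors the left-hand mesh.
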(event OnComponentBeginOverlap(GrabCollision)
  (params (OverlappedComponent :type Primitive%20Component%20Object%20Reference) (OtherActor :type Actor%20Object%20Reference) (OtherComp :type Primitive%20Component%20Object%20Reference) (OtherBodyIndex :type Integer) (bFromSweep :type Boolean) (SweepResult :type Hit%20Result%20Structure%20%28by%20ref%29))
  (bind _returnvalue (Actor|GetComponentbyClass OtherActor "/Game/StartOculusTouch/Blueprints/BPC_GrabTarget.BPC_GrabTarget_C"))
  ;[1 1 1] Begin Overlap GrabCollision
  (Utilities|IsValid _returnvalue
    (:Is%20Valid
      (if (not (Utilities|Array|ContainsItem (Variables|Default|GetGrabTargetComponents) _returnvalue))
        (Utilities|Array|Add (Variables|Default|GetGrabTargetComponents) _returnvalue)
        (Game|AssignOnDestroyed OtherActor (delegate Custom|OnDestroyed_Event_0))))))

(event OnComponentEndOverlap(GrabCollision)
  (params (OverlappedComponent :type Primitive%20Component%20Object%20Reference) (OtherActor :type Actor%20Object%20Reference) (OtherComp :type Primitive%20Component%20Object%20Reference) (OtherBodyIndex :type Integer))
  (bind _returnvalue (Actor|GetComponentbyClass OtherActor "/Game/StartOculusTouch/Blueprints/BPC_GrabTarget.BPC_GrabTarget_C"))
  ;[1 1 1] End Overlap GrabCollision
  (Utilities|IsValid _returnvalue
    (:Is%20Valid
      (Utilities|Array|RemoveItem (Variables|Default|GetGrabTargetComponents) _returnvalue)
      (Default|NotTargeted _returnvalue self))))

(event Custom|PlayHapticEffect
  (params (HapticEffect :type Haptic%20Feedback%20Effect%20Base%20Object%20Reference) (Scale :type Float%20%28single-precision%29) (bLoop :type Boolean))
  ;[1 1 1] Haptic Effect
  (Class|PlayerController|PlayHapticEffect (Game|GetPlayerController 0) HapticEffect (Variables|Default|GetHand) Scale bLoop))

(event Custom|Release%20By%20OtherHand
  ;[1 1 1] Release By OtherHand
  (Variables|Default|SetGrabingComponent 0)
  (Rendering|SetVisibility (Variables|Default|GetHandMesh) true false))

(event Custom|StopHapticEffect
  ;[1 1 1] Haptic Effect
  (Class|PlayerController|StopHapticEffect (Game|GetPlayerController 0) (Variables|Default|GetHand)))

(event Custom|SetHaptics%20byValue
  (params (Frequency :type Float%20%28single-precision%29) (Amplitude :type Float%20%28single-precision%29))
  ;[1 1 1] Haptic Effect
  (Class|PlayerController|SetHapticsbyValue (Game|GetPlayerController 0) Frequency Amplitude (Variables|Default|GetHand)))

(event Custom|OnDestroyed_Event_0
  (params (DestroyedActor :type Actor%20Object%20Reference))
  ;[1 1 1] Begin Overlap GrabCollision
  (Utilities|Array|RemoveItem (Variables|Default|GetGrabTargetComponents) (Actor|GetComponentbyClass DestroyedActor "/Game/StartOculusTouch/Blueprints/BPC_GrabTarget.BPC_GrabTarget_C")))

(event EventTick
  (params (DeltaSeconds :type Float%20%28single-precision%29))
  ;[1 1 1] Tick
  (CallFunction|UpdateGrabCollisionRotation)
  (CallFunction|UpdateGrabTargettingComponent))

(event Custom|Update%20Grab%20Collision%20Rotation
  ;[1 1 1] Update Grab Collision
  (Transformation|SetWorldRotation (Variables|Default|GetGrabCollisionRoot) (Math|Rotator|FindLookatRotation (Utilities|GetCameraLocation) (Transformation|GetWorldLocation (Variables|Default|GetGrabCollisionRoot))) false false))

(event Custom|Update%20Grab%20Targetting%20Component
  ;[1 1 1] Update Grab Target
  (if (and (not (Utilities|IsValid (Variables|Default|GetGrabingComponent))) (> (Utilities|Array|Length (Variables|Default|GetGrabTargetComponents)) 0))
    (bind _result (CallFunction|GetNearestComponent (Variables|Default|GetGrabTargetComponents)))
    (Utilities|FlowControl|Sequence
      (:then_0
        (if (and (Utilities|IsValid (Variables|Default|GetGrabTargetingComponent)) (!= (Variables|Default|GetGrabTargetingComponent) _result))
          (Default|NotTargeted (Variables|Default|GetGrabTargetingComponent) self)))
      (:then_1
        (bind _output_get (Variables|Default|SetGrabTargetingComponent _result))
        (Default|Targeted _output_get self)))
    (else
      (Variables|Default|SetGrabTargetingComponent 0))))

(event EventRelease
  ;[1 1 1] Release Action
  (Utilities|IsValid (Variables|Default|GetGrabingComponent)
    (:Is%20Valid
      (Default|Released (Variables|Default|GetGrabingComponent) self)
      (Variables|Default|SetGrabingComponent 0)
      (Rendering|SetVisibility (Variables|Default|GetHandMesh) true false))))

(event EventStartUse
  (bind _grabingcomponent (Variables|Default|GetGrabingComponent))
  ;[1 1 1] Stop Use Action
  (Utilities|IsValid _grabingcomponent
    (:Is%20Valid
      (Default|StartUsed _grabingcomponent))))

(event EventStopUse
  (bind _grabingcomponent (Variables|Default|GetGrabingComponent))
  ;[1 1 1] Stop Used
  (Utilities|IsValid _grabingcomponent
    (:Is%20Valid
      (Default|StopUsed _grabingcomponent))))

(event EventPressThumbStick
  (bind _grabingcomponent (Variables|Default|GetGrabingComponent))
  ;[1 1 1] Thumb Stick
  (Utilities|IsValid _grabingcomponent
    (:Is%20Valid
      (Default|PressThumbStick _grabingcomponent))))

(event EventReleaseThumbStick
  (bind _grabingcomponent (Variables|Default|GetGrabingComponent))
  ;[1 1 1] Thumb Stick
  (Utilities|IsValid _grabingcomponent
    (:Is%20Valid
      (Class|BPIOculusTouch|ReleaseThumbStick(Message) _grabingcomponent))))

(event EventStartThumbUp
  ;[1 1 1] Thumb Up
  (Utilities|Struct|SetmembersinStruct_OculusTouchInput (Variables|OculusTouch|GetOculusTouchInputData) true))

(event EventStopThumpUp
  ;[1 1 1] Thumb Up
  (Utilities|Struct|SetmembersinStruct_OculusTouchInput (Variables|OculusTouch|GetOculusTouchInputData) false))

(event EventStartPointing
  ;[1 1 1] Pointing
  (Utilities|Struct|SetmembersinStruct_OculusTouchInput (Variables|OculusTouch|GetOculusTouchInputData) true))

(event EventStopPointing
  ;[1 1 1] Pointing
  (Utilities|Struct|SetmembersinStruct_OculusTouchInput (Variables|OculusTouch|GetOculusTouchInputData) false))

(event EventPressTouchButton1
  (bind _grabingcomponent (Variables|Default|GetGrabingComponent))
  ;[1 1 1] Touch Button 1
  (Utilities|IsValid _grabingcomponent
    (:Is%20Valid
      (Default|PressButton1 _grabingcomponent))))

(event EventReleaseTouchButton1
  (bind _grabingcomponent (Variables|Default|GetGrabingComponent))
  ;[1 1 1] Touch Button 1
  (Utilities|IsValid _grabingcomponent
    (:Is%20Valid
      (Default|ReleaseButton1 _grabingcomponent))))

(event EventReleaseTouchButton2
  (bind _grabingcomponent (Variables|Default|GetGrabingComponent))
  ;[1 1 1] Touch Button 2
  (Utilities|IsValid _grabingcomponent
    (:Is%20Valid
      (Default|ReleaseButton2 _grabingcomponent))))

(event EventSetTriggerRateIndex
  (params (rate :type Float%20%28single-precision%29))
  ;[1 1 1] Trigger / Stick
  (Utilities|Struct|SetmembersinStruct_OculusTouchInput (Variables|OculusTouch|GetOculusTouchInputData) rate))

(event EventSetTriggerRateOther
  (params (rate :type Float%20%28single-precision%29))
  ;[1 1 1] Trigger / Stick
  (Utilities|Struct|SetmembersinStruct_OculusTouchInput (Variables|OculusTouch|GetOculusTouchInputData) rate))

(event EventSetThumbStickAxisX
  (params (Axis%20Value :type Float%20%28single-precision%29))
  ;[1 1 1] Trigger / Stick
  (Utilities|Struct|SetmembersinStruct_OculusTouchInput (Variables|OculusTouch|GetOculusTouchInputData) Axis%20Value))

(event EventPressTouchButton2
  (bind _grabingcomponent (Variables|Default|GetGrabingComponent))
  ;[1 1 1] Touch Button 2
  (Utilities|IsValid _grabingcomponent
    (:Is%20Valid
      (Default|PressButton2 _grabingcomponent))))

(event EventSetThumbStickAxisY
  (params (Axis%20Value :type Float%20%28single-precision%29))
  ;[1 1 1] Trigger / Stick
  (Utilities|Struct|SetmembersinStruct_OculusTouchInput (Variables|OculusTouch|GetOculusTouchInputData) Axis%20Value))

(event EventGrab
  (bind _grabtargetingcomponent (Variables|Default|GetGrabTargetingComponent))
  ;[1 1 1] Grab Action
  (Utilities|IsValid _grabtargetingcomponent
    (:Is%20Valid
      (bind _output_get (Variables|Default|SetGrabingComponent _grabtargetingcomponent))
      (Default|Grabed _output_get self)
      (Default|NotTargeted (Variables|Default|GetGrabTargetingComponent) self)
      (Rendering|SetVisibility (Variables|Default|GetHandMesh) false false))))

(fn ConstructionScript
  (Variables|/Script/HeadMountedDisplay.MotionControllerComponent|SetHand (Variables|Default|GetMotionController) (Variables|Default|GetHand))
  (Utilities|FlowControl|Sequence
    (:then_0
      ;[0 0 0] 左手の場合はメッシュを反転させる
      (switch Utilities|FlowControl|Switch|SwitchonEControllerHand (Variables|Default|GetHand)
        (:Left
          (Transformation|SetWorldScale3D (Variables|Default|GetHandMesh) "1.000000,1.000000,-1.000000"))))
    (:then_1
      (CallFunction|UpdateGrabCollisionSize (Variables|Default|GetGrabCollisionData)))))

(fn UpdateGrabCollisionSize
  (params (CollisionParam :type Struct%20Box%20Collision%20Param%20Structure))
  (bind _output_get (Variables|Default|SetGrabCollisionData CollisionParam))
  (Utilities|FlowControl|Sequence
    (:then_0
      (Components|Box|SetBoxExtent (Variables|Default|GetGrabCollision) (* (Math|Vector|MakeVector (.Length (Utilities|Struct|BreakStruct_BoxCollisionParam _output_get)) (.Width (Utilities|Struct|BreakStruct_BoxCollisionParam _output_get)) (.Height (Utilities|Struct|BreakStruct_BoxCollisionParam _output_get))) 0.5) true))
    (:then_1
      (Transformation|SetRelativeLocation (Variables|Default|GetGrabCollision) (Math|Vector|MakeVector (* (.Length (Utilities|Struct|BreakStruct_BoxCollisionParam _output_get)) 0.5) 0.0 0.0) false false))))

(fn GetNearestComponent
  (params (Comps :type Array%20of%20BPC%20Grab%20Target%20Object%20References))
  (for _array_element Comps
    (Utilities|IsValid _array_element
      (:Is%20Valid
        (if (< (Math|Vector|VectorLength (- (Transformation|GetActorLocation (Components|GetOwner _array_element)) (Transformation|GetActorLocation))) (LocalVariables|Getlength))
          (LocalVariables|SetoutComp _array_element)
          (LocalVariables|Setlength (Math|Vector|VectorLength (- (Transformation|GetActorLocation (Components|GetOwner _array_element)) (Transformation|GetActorLocation))))))))
  (return (LocalVariables|GetoutComp)))

(fn GetOculusTouchInputData
  (return (Variables|OculusTouch|GetOculusTouchInputData)))
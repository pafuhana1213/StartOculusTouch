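; BPC_MotionControllerManager is a component that spawns and tracks the left and right VR hand controllers.
; SpawnMotionControllers creates a BP_MotionController per hand, owned by the component's owner and snapped to the given parent component.
; Both references are stored for lookup by hand type through GetMotionController.
; Without an enabled HMD, each hand is offset forward and sideways for gamepad debugging.
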(event Custom|Spawn%20Motion%20Controllers
  (params (Parent :type Scene%20Component%20Object%20Reference))
  ;[1 1 1] モーションコントローラの生成
  (Utilities|FlowControl|Sequence
    (:then_0
      (CallFunction|SpawnMotionController "Left" Parent))
    (:then_1
      (CallFunction|SpawnMotionController "Right" Parent))))

(fn SpawnMotionController
  (params (Type :type EControllerHand%20Enum) (Parent :type Scene%20Component%20Object%20Reference))
  ;[1 1 1] 手用のBP生成
  (bind _returnvalue (Game|SpawnActorfromClass "/Game/StartOculusTouch/Blueprints/BP_MotionController.BP_MotionController_C" (Math|Transform|MakeTransform "0, 0, 0" "0, 0, 0" "1,1,1") "AlwaysSpawn" (Components|GetOwner) Type 0)) ; 手用のBPを生成
  (Utilities|FlowControl|Sequence
    (:then_0
      ;[1 1 1] VRの座標系に
      (Transformation|AttachComponentToComponent _returnvalue Parent "None" "SnapToTarget" "SnapToTarget" "KeepWorld" false))
    (:then_1
      ;[1 1 1] 右手・左手用BPを保存
      (switch Utilities|FlowControl|Switch|SwitchonEControllerHand Type
        (:Left
          (bind _output_get (Variables|Default|SetLeftController _returnvalue))
          ;[1 1 1] ゲームパッドを使ったデバッグ用オフセット
          (if (not (Class|HeadMountedDisplayFunctionLibrary|IsHeadMountedDisplayEnabled))
            (Transformation|AddActorWorldOffset _output_get "50.000000,-30.000000,0.000000")))
        (:Right
          (bind _output_get_2 (Variables|Default|SetRightController _returnvalue))
          (if (not (Class|HeadMountedDisplayFunctionLibrary|IsHeadMountedDisplayEnabled))
            (Transformation|AddActorWorldOffset _output_get_2 "50.000000,30.000000, 0")))))))

(fn GetMotionController
  (params (Type :type EControllerHand%20Enum))
  (return (Utilities|Select :Index Type :Left (Variables|Default|GetLeftController) :Right (Variables|Default|GetRightController) :Pad 0 :ExternalCamera 0 :Special_1 0 :Special_2 0 :Special_3 0 :Special_4 0 :Special_5 0 :Special_6 0 :Special_7 0 :Special_8 0 :Special_9 0)))
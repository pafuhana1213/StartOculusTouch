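; Child grab-sample actor for motion controllers that eases toward the controller holding it instead of snapping to it.
; On grab it calls CheckExchange, turns off mesh physics simulation and stores the grabbing controller.
; While that reference is valid, Tick interpolates location and rotation toward the controller, offset by the inverse of BPCGrabTarget's relative transform, with separate speeds for each.
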(event EventBeginPlay
  (|CallParentFunction))

(event EventGrabed
  (params (MotionController :type BP%20Motion%20Controller%20Object%20Reference))
  (Utilities|FlowControl|Sequence
    (:then_0
      (CallFunction|CheckExchange MotionController)
      (Physics|SetSimulatePhysics (Variables|Default|GetStaticMesh) false))
    (:then_1
      (Variables|Default|SetGrabMotionController MotionController))))

(event EventTick
  (params (DeltaSeconds :type Float%20%28single-precision%29))
  (bind _returnvalue (Transformation|GetActorTransform))
  (bind _returnvalue_2 (Utilities|Time|GetWorldDeltaSeconds))
  (bind _bpc_grabtarget (Variables|Default|GetBPC_GrabTarget))
  (bind _grabmotioncontroller (Variables|Default|GetGrabMotionController))
  (bind _returnvalue_3 (Transformation|GetActorTransform _grabmotioncontroller))
  (bind _returnvalue_4 (Transformation|GetRelativeTransform _bpc_grabtarget))
  (bind _returnvalue_5 (Math|Transform|InvertTransform _returnvalue_4))
  (Utilities|IsValid (Variables|Default|GetGrabMotionController)
    (:Is%20Valid
      (Transformation|SetActorTransform (Math|Transform|MakeTransform (Math|Interpolation|VInterpTo (.location _returnvalue) (+ (.location _returnvalue_3) (.location _returnvalue_5)) _returnvalue_2 (Variables|Default|GetLocationInterpSpeed)) (Math|Interpolation|RInterpTo (.rotation _returnvalue) (Math|Rotator|CombineRotators (.rotation _returnvalue_3) (.rotation _returnvalue_5)) _returnvalue_2 (Variables|Default|GetRotationInterpSpeed)) (.scale _returnvalue))))))

(fn ConstructionScript
  (|CallParentFunction))
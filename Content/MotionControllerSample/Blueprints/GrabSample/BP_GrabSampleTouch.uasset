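; BP_GrabSampleTouch is a grabbable sample object that drives a target character from the Oculus Touch controller holding it.
; Each Tick it caches the grabbing motion controller's thumbstick axes and moves a debug sphere to mirror the tilt.
; The left hand moves the character along its dominant stick axis, forward or sideways, while the right hand yaws it over time.
; Using the object makes the character jump.
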(event Custom|UpdateSphereTransform
  ;[1 1 1] スティックの傾きに応じて玉を移動(デバッグ用)
  (switch Utilities|FlowControl|Switch|SwitchonEControllerHand (Variables|/Game/MotionControllerSample/Blueprints/BP_MotionController.BP_MotionController_C|GetHand (Variables|Default|GetGrabMotionController))
    (:Left
      (Transformation|SetRelativeLocation (Variables|Default|GetSphere) (Math|Vector|MakeVector (Variables|Default|GetThumbStickY) (* (.z (Transformation|GetActorScale3D)) (Variables|Default|GetThumbStickX)) 0.0) false false))
    (:Right
      (Transformation|SetRelativeLocation (Variables|Default|GetSphere) (Math|Vector|MakeVector (Variables|Default|GetThumbStickY) (* (.z (Transformation|GetActorScale3D)) (Variables|Default|GetThumbStickX)) 0.0) false false))))

(event Custom|OperateTutorialCharacter
  (bind _targetcharacter (Variables|Default|GetTargetCharacter))
  (bind _targetcharacter_2 (Variables|Default|GetTargetCharacter))
  ;[1 1 1] キャラクターの移動操作
  (Utilities|IsValid (Variables|Default|GetTargetCharacter)
    (:Is%20Valid
      (switch Utilities|FlowControl|Switch|SwitchonEControllerHand (Variables|/Game/MotionControllerSample/Blueprints/BP_MotionController.BP_MotionController_C|GetHand (Variables|Default|GetGrabMotionController))
        (:Left
          (Math|Float|CompareFloat (Math|Float|Absolute(Float) (Variables|Default|GetThumbStickY)) (Math|Float|Absolute(Float) (Variables|Default|GetThumbStickX))
            (:>
              (Pawn|Input|AddMovementInput _targetcharacter_2 (Transformation|GetActorForwardVector _targetcharacter_2) (Variables|Default|GetThumbStickY) false :!label _label))
            (:==
              (goto _label))
            (:<
              (Pawn|Input|AddMovementInput _targetcharacter (Transformation|GetActorRightVector _targetcharacter) (Variables|Default|GetThumbStickX) false))))
        (:Right
          (Class|Actor|AddActorWorldRotation (Variables|Default|GetTargetCharacter) (Math|Rotator|MakeRotator 0.0 0.0 (* (Variables|Default|GetThumbStickX) (Utilities|Time|GetWorldDeltaSeconds) 1e+02))))))))

(event EventTick
  (params (DeltaSeconds :type Float%20%28single-precision%29))
  (bind _grabmotioncontroller (Variables|Default|GetGrabMotionController))
  (bind _oculustouchinputdata (Variables|/Game/MotionControllerSample/Blueprints/BP_MotionController.BP_MotionController_C|GetOculusTouchInputData _grabmotioncontroller))
  (Utilities|IsValid (Variables|Default|GetGrabMotionController)
    (:Is%20Valid
      (Utilities|FlowControl|Sequence
        (:then_0
          ;[1 1 1] スティックの傾きを保存
          (Variables|Default|SetThumbStickX (.thumbstickaxisx _oculustouchinputdata))
          (Variables|Default|SetThumbStickY (.thumbstickaxisy _oculustouchinputdata)))
        (:then_1
          (CallFunction|UpdateSphereTransform)
          (CallFunction|OperateTutorialCharacter))))))

(event EventStartUsed
  (params (MotionController :type BP%20Motion%20Controller%20Object%20Reference))
  (bind _targetcharacter (Variables|Default|GetTargetCharacter))
  (Utilities|IsValid _targetcharacter
    (:Is%20Valid
      (Character|Jump _targetcharacter))))

(event EventPressThumbStick
  (params (MotionController :type BP%20Motion%20Controller%20Object%20Reference)))

(event EventReleaseThumbStick
  (params (MotionController :type BP%20Motion%20Controller%20Object%20Reference)))

(fn ConstructionScript
  (|CallParentFunction))
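; Base grabbable actor for the motion controller sample, handling grab, hand-to-hand exchange and release.
; It binds to BPCGrabTarget dispatchers; grabbing releases any other hand, attaches to the controller offset by the grab target's inverse transform, and pulses haptics.
; Release detaches and enables mesh physics; use events are empty stubs.
; A dynamic material created at construction highlights the object while targeted.
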(event Custom|Bind%20StartUsed
  ;[1 1 1] Start Used
  (EventDispatchers|AssignEDStartUsed (Variables|Default|GetBPC_GrabTarget) (delegate Custom|StartUsed)))

(event Custom|Bind%20StopUsed
  ;[1 1 1] Stop Used
  (EventDispatchers|AssignEDStopUsed (Variables|Default|GetBPC_GrabTarget) (delegate Custom|StopUsed)))

(event Custom|Bind%20Targeted
  ;[1 1 1] Targeted
  (EventDispatchers|AssignEDTargeted (Variables|Default|GetBPC_GrabTarget) (delegate Custom|Targeted)))

(event Custom|Bind%20NotTargeted
  ;[1 1 1] Not Targeted
  (EventDispatchers|AssignEDNotTargeted (Variables|Default|GetBPC_GrabTarget) (delegate Custom|NotTargeted)))

(event Custom|StopUsed
  (params (MotionController :type BP%20Motion%20Controller%20Object%20Reference))
  ;[1 1 1] Stop Used
)

(event Custom|HapticEffectGrabed
  (bind _grabmotioncontroller (Variables|Default|GetGrabMotionController))
  ;[1 1 1] Haptic Effect for Grabed
  (Utilities|IsValid _grabmotioncontroller
    (:Is%20Valid
      (Default|SetHapticsbyValue _grabmotioncontroller 3.2e+02 0.2)
      (Utilities|FlowControl|Delay 0.1)
      (Utilities|IsValid _grabmotioncontroller
        (:Is%20Valid
          (Default|SetHapticsbyValue _grabmotioncontroller 3.2e+02 0.0))))))

(event Custom|Grabed
  (params (MotionController :type BP%20Motion%20Controller%20Object%20Reference))
  (bind _bpc_grabtarget (Variables|Default|GetBPC_GrabTarget))
  (bind _returnvalue (Transformation|GetRelativeTransform _bpc_grabtarget))
  (bind _returnvalue_2 (Math|Transform|InvertTransform _returnvalue))
  ;[1 1 1] Grabed
  (Utilities|FlowControl|Sequence
    (:then_0
      (CallFunction|CheckExchange MotionController))
    (:then_1
      (bind _output_get (Variables|Default|SetGrabMotionController MotionController))
      (Transformation|AttachActorToActor _output_get "None" "SnapToTarget" "SnapToTarget" "KeepRelative" true)
      (Class|Actor|AddActorLocalTransform (Math|Transform|MakeTransform (.location _returnvalue_2) (.rotation _returnvalue_2) "1.000000,1.000000,1.000000") false false))
    (:then_2
      (CallFunction|HapticEffectGrabed))))

(event Custom|Released
  (params (MotionController :type BP%20Motion%20Controller%20Object%20Reference))
  ;[1 1 1] Released
  (Transformation|DetachFromActor "KeepRelative" "KeepRelative" "KeepRelative")
  (Physics|SetSimulatePhysics (Variables|Default|GetStaticMesh) true)
  (Variables|Default|SetGrabMotionController 0))

(event Custom|StartUsed
  (params (MotionController :type BP%20Motion%20Controller%20Object%20Reference))
  ;[1 1 1] Start Used
)

(event Custom|Bind%20Released
  ;[1 1 1] Released
  (EventDispatchers|AssignEDReleased (Variables|Default|GetBPC_GrabTarget) (delegate Custom|Released)))

(event Custom|Targeted
  (params (MotionController :type BP%20Motion%20Controller%20Object%20Reference))
  ;[1 1 1] Targeted
  (Rendering|Material|SetScalarParameterValue (Variables|Default|GetMaterial) "IsTargeted" 1.0 :!class /Script/Engine.MaterialInstanceDynamic))

(event Custom|NotTargeted
  (params (MotionController :type BP%20Motion%20Controller%20Object%20Reference))
  ;[1 1 1] Not Targeted
  (Rendering|Material|SetScalarParameterValue (Variables|Default|GetMaterial) "IsTargeted" 0.0 :!class /Script/Engine.MaterialInstanceDynamic))

(event Custom|Bind%20Grabed
  ;[1 1 1] Grabed
  (EventDispatchers|AssignEDGrabed (Variables|Default|GetBPC_GrabTarget) (delegate Custom|Grabed)))

(event Custom|Bind%20Events
  ;[1 1 1] Bind Eventes
  (CallFunction|BindGrabed)
  (CallFunction|BindReleased)
  (CallFunction|BindStartUsed)
  (CallFunction|BindStopUsed)
  (CallFunction|BindTargeted)
  (CallFunction|BindNotTargeted))

(event EventBeginPlay
  ;[1 1 1] BeginPlay
  (CallFunction|BindEvents))

(fn ConstructionScript
  (bind _returnvalue (Rendering|Material|CreateDynamicMaterialInstance (Variables|Default|GetStaticMesh) 0 "/Game/MotionControllerSample/Material/M_GrabTarget.M_GrabTarget" :!class /Script/Engine.PrimitiveComponent))
  (Variables|Default|SetMaterial _returnvalue))

(fn CheckExchange
  (params (MotionController :type BP%20Motion%20Controller%20Object%20Reference))
  (bind _grabmotioncontroller (Variables|Default|GetGrabMotionController))
  (if (and (!= MotionController _grabmotioncontroller) (Utilities|IsValid _grabmotioncontroller))
    (Default|ReleasebyOtherHand (Variables|Default|GetGrabMotionController))
    (return true)
    (else
      (return false))))
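; BP_GrabSample is a sample grabbable actor for motion controllers, driven by events from its BPCGrabTarget component.
; On grab, it makes any previous controller release, snaps onto the new one and applies the inverse of the grab target's relative transform to align the grip point.
; On release, it enables mesh physics and clears the stored controller.
; Used, Targeted and NotTargeted handlers are bound but empty.
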(event Custom|ED_Grabed_Event_0
  (params (MotionController :type BP%20Motion%20Controller%20Object%20Reference))
  (bind _bpc_grabtarget (Variables|Default|GetBPC_GrabTarget))
  (bind _returnvalue (Transformation|GetRelativeTransform _bpc_grabtarget))
  (bind _returnvalue_2 (Math|Transform|InvertTransform _returnvalue))
  ;[1 1 1] Grabed
  (Utilities|FlowControl|Sequence
    (:then_0
      (if (and (!= MotionController (Variables|Default|GetGrabMotionController)) (Utilities|IsValid (Variables|Default|GetGrabMotionController)))
        (Default|ReleasebyOtherHand (Variables|Default|GetGrabMotionController))))
    (:then_1
      (bind _output_get (Variables|Default|SetGrabMotionController MotionController))
      (Transformation|AttachActorToActor _output_get "None" "SnapToTarget" "SnapToTarget" "KeepRelative" true)
      (Class|Actor|AddActorLocalTransform (Math|Transform|MakeTransform (.location _returnvalue_2) (.rotation _returnvalue_2) "1.000000,1.000000,1.000000") false false))))

(event Custom|ED_Released_Event_0
  (params (MotionController :type BP%20Motion%20Controller%20Object%20Reference))
  ;[1 1 1] Released
  (Transformation|AttachActorToActor 0 "None" "KeepRelative" "KeepRelative" "KeepRelative" true)
  (Physics|SetSimulatePhysics (Variables|Default|GetStaticMesh) true)
  (Variables|Default|SetGrabMotionController 0))

(event Custom|ED_Used_Event_0
  (params (MotionController :type BP%20Motion%20Controller%20Object%20Reference))
  ;[1 1 1] Used
)

(event Custom|ED_Targeted_Event_0
  (params (MotionController :type BP%20Motion%20Controller%20Object%20Reference))
  ;[1 1 1] Targeted
)

(event Custom|ED_NotTargeted_Event_0
  (params (MotionController :type BP%20Motion%20Controller%20Object%20Reference))
  ;[1 1 1] NotTargeted
)

(event Custom|Bind%20Events
  (Utilities|FlowControl|Sequence
    (:then_0
      ;[1 1 1] Grabed
      (EventDispatchers|AssignEDGrabed (Variables|Default|GetBPC_GrabTarget) (delegate Custom|ED_Grabed_Event_0)))
    (:then_1
      ;[1 1 1] Released
      (EventDispatchers|AssignEDReleased (Variables|Default|GetBPC_GrabTarget) (delegate Custom|ED_Released_Event_0)))
    (:then_2
      ;[1 1 1] Used
      (EventDispatchers|AssignEDUsed (Variables|Default|GetBPC_GrabTarget) (delegate Custom|ED_Used_Event_0)))
    (:then_3
      ;[1 1 1] Targeted
      (EventDispatchers|AssignEDTargeted (Variables|Default|GetBPC_GrabTarget) (delegate Custom|ED_Targeted_Event_0)))
    (:then_4
      ;[1 1 1] NotTargeted
      (EventDispatchers|AssignEDNotTargeted (Variables|Default|GetBPC_GrabTarget) (delegate Custom|ED_NotTargeted_Event_0)))))

(event EventBeginPlay
  (CallFunction|BindEvents))

(fn ConstructionScript)
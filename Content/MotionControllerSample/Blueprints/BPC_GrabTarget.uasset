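; BPC_GrabTarget is a grab-target component from the motion controller sample that relays interaction events through event dispatchers.
; Grab and release update the grabbed flag and stored controller reference, and broadcast the controller involved.
; Use, button and thumbstick events rebroadcast with the stored grabbing controller.
; Targeted and untargeted events simply forward the controller they receive.
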(event Custom|Grabed
  (params (MotionController :type BP%20Motion%20Controller%20Object%20Reference))
  ;[1 1 1] Grabed
  (Default|CallEDGrabed MotionController)
  (Variables|Default|SetIsGrabed true)
  (Variables|Default|SetGrabMotionController MotionController))

(event Custom|PressThumbStick
  ;[1 1 1] ThumbStick
  (Default|CallEDPressThumbStick (Variables|Default|GetGrabMotionController)))

(event Custom|Targeted
  (params (MotionController :type BP%20Motion%20Controller%20Object%20Reference))
  ;[1 1 1] Targeted
  (Default|CallEDTargeted MotionController))

(event Custom|ReleaseThumbStick
  ;[1 1 1] ThumbStick
  (Default|CallEDReleaseThumbStick (Variables|Default|GetGrabMotionController)))

(event Custom|NotTargeted
  (params (MotionController :type BP%20Motion%20Controller%20Object%20Reference))
  ;[1 1 1] NotTargeted
  (Default|CallEDNotTargeted MotionController))

(event Custom|Stop%20Used
  ;[1 1 1] Stop Used
  (Default|CallEDStopUsed (Variables|Default|GetGrabMotionController)))

(event Custom|Press%20Button%201
  ;[1 1 1] Button1
  (Default|CallEDPressButton1 (Variables|Default|GetGrabMotionController)))

(event Custom|Release%20Button%201
  ;[1 1 1] Button1
  (Default|CallEdReleaseButton1 (Variables|Default|GetGrabMotionController)))

(event Custom|Released
  (params (MotionController :type BP%20Motion%20Controller%20Object%20Reference))
  ;[1 1 1] Released
  (Default|CallEDReleased MotionController)
  (Variables|Default|SetIsGrabed false)
  (Variables|Default|SetGrabMotionController 0))

(event Custom|Press%20Button%202
  ;[1 1 1] Button 2
  (Default|CallEDPressButton2 (Variables|Default|GetGrabMotionController)))

(event Custom|Release%20Button%202
  ;[1 1 1] Button 2
  (Default|CallEDReleaseButton2 (Variables|Default|GetGrabMotionController)))

(event Custom|Start%20Used
  ;[1 1 1] Start Used
  (Default|CallEDStartUsed (Variables|Default|GetGrabMotionController)))